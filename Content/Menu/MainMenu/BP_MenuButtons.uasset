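; BP_MenuButtons is a clickable main menu button built from a mesh, collision and text label, with a configurable caption and target widget.
; The construction script applies the caption, and BeginPlay creates the widget from the assigned class.
; Cursor events on the collision swap the mesh material and play a sound on hover.
; Releasing a click passes the widget to HUD_MainMenu for display.
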(event `self.ReceiveBeginPlay`
  (bind _returnvalue (`|CreateWidget` (`self.Widget Class`)))
  (set `self.Widget` _returnvalue))

(event `self.Mesh Collision.OnBeginCursorOver`
  (params (TouchedComponent :type "PrimitiveComponent Object Reference"))
  (`PrimitiveComponent.SetMaterial` (`self.Mesh`) 0 "/Engine/EngineMeshes/BackgroundMaterial.BackgroundMaterial")
  (`GameplayStatics.PlaySound2D` "/Engine/VREditor/Sounds/UI/Selection_Changes.Selection_Changes" 1.0 1.0 0.0 null null))

(event `self.Mesh Collision.OnEndCursorOver`
  (params (TouchedComponent :type "PrimitiveComponent Object Reference"))
  (`PrimitiveComponent.SetMaterial` (`self.Mesh`) 0 "/Engine/BasicShapes/BasicShapeMaterial.BasicShapeMaterial"))

(event `self.Mesh Collision.OnReleased`
  (params (TouchedComponent :type "PrimitiveComponent Object Reference") (ButtonReleased :type "Key Structure"))
  (bind _ashud_main_menu (cast `/Game/Menu/MainMenu/Widgets/HUD_MainMenu` (`PlayerController.GetHUD` (`GameplayStatics.GetPlayerController` 0))))
  (`/Game/Menu/MainMenu/Widgets/HUD_MainMenu.Display Widget` _ashud_main_menu (`self.Widget`)))

(fn `UserConstructionScript`
  (`TextRenderComponent.K2_SetText` (`self.Button Name`) (`self.Text`)))