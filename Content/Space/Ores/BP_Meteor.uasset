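; BP_Meteor is a mineable space ore that drops items as it takes damage.
; On construction it rolls health as a random number of fixed-HP units and creates a WG_Meteor health widget, shown while looked at.
; Damage spawns one BP_Drop per depleted unit and updates the widget, while the final blow spawns a larger batch.
; On destruction it frees its parent spawn point and notifies the game mode.
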(event `/Game/Space/Player/BPI_Interactable.Damage`
  (params (Damage :type Integer))
  (`self.Apply Damage` Damage))

(event `self.ReceiveDestroyed`
  (set `/Game/Space/Ores/BP_MeteorSpawnPoint.IsOccupied` false (`self.Parent Spawn Point`))
  (message `/Game/Space/Level/BPI_MapEvents.Ore Destruction` (`GameplayStatics.GetGameMode`)))

(event `/Game/Space/Player/BPI_Interactable.Look`
  (`Widget.SetVisibility` (`self.Meteor Widget`) "Visible"))

(event `/Game/Space/Player/BPI_Interactable.EndLook`
  (`Widget.SetVisibility` (`self.Meteor Widget`) "Hidden"))

(fn `Apply Damage`
  (params (Damage :type Integer))
  (if (!= (`KismetMathLibrary.Clamp` (- (`self.Current HP`) (`local.Damage`)) 0 (`self.Max Meteor HP`)) 0)
    (for _ (range 1 (+ (/ (+ (mod (- (`self.Max Meteor HP`) (`self.Current HP`)) (`self.Max Unit Hp`)) (`local.Damage`)) (`self.Max Unit Hp`)) 1))
      (`self.Spawn Loot Function`))
    (`/Game/Space/Ores/Widgets/WG_Meteor.Take Damage` (`self.Meteor Widget`) (/ (`local.Damage`) (`self.Max Unit Hp`)) (/ (`self.Get Current Unit HP`) (`self.Max Unit Hp`)))
    (set `self.Current HP` (`KismetMathLibrary.Clamp` (- (`self.Current HP`) (`local.Damage`)) 0 (`self.Max Meteor HP`)))
    (else
      ; Destroy
      (set `self.Current HP` 0)
      (for _ (range 1 (+ (+ (/ (/ (`self.Max Meteor HP`) (`self.Max Unit Hp`)) 2) (`self.Min Unit Quantity`)) 1))
        (`self.Spawn Loot Function`))
      (`self.K2_DestroyActor`))))

(fn `Create Widget`
  (bind _returnvalue (`|CreateWidget` "/Game/Space/Ores/Widgets/WG_Meteor.WG_Meteor_C"))
  (bind _output_get (set `self.Meteor Widget` _returnvalue))
  (`/Game/Space/Ores/Widgets/WG_Meteor.Set Widget` _output_get (`self.Meteor Name`) (`self.Max Meteor HP`) (`self.Current HP`) (`self.Max Unit Hp`) (`self.Get Current Unit HP`) (`self.Meteor Color`))
  (`WidgetComponent.SetWidget` (`self.Widget`) (`self.Meteor Widget`)))

(fn `Get Current Unit HP`
  (returns (`Unit HP` :type Integer))
  (return (- (`self.Max Unit Hp`) (mod (- (`self.Max Meteor HP`) (`self.Current HP`)) (`self.Max Unit Hp`)))))

(fn `Set Health Points`
  (bind _output_get (set `self.Max Meteor HP` (* (`KismetMathLibrary.RandomIntegerInRange` (`self.Min Unit Quantity`) (`self.Max Unit Quantity`)) (`self.Max Unit Hp`))))
  (set `self.Current HP` _output_get))

(fn `Spawn Loot Function`
  (bind _returnvalue (`|SpawnActorFromClass` "/Game/Space/Ores/BP_Drop.BP_Drop_C" (`self.GetTransform`) "AlwaysSpawn" "MultiplyWithRoot" null null))
  (`/Game/Space/Ores/BP_Drop.ItemDrop` _returnvalue 1 (`self.Droping Item`)))

(fn `Update Widget Health`
  (`/Game/Space/Ores/Widgets/WG_Meteor.Update Health` (`self.Meteor Widget`) (`self.Max Meteor HP`) (`self.Current HP`) (`self.Max Unit Hp`) (`self.Get Current Unit HP`)))

(fn `UserConstructionScript`
  (`self.Set Health Points`)
  (`self.Create Widget`))