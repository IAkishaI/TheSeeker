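; Dropped item pickup for the space game's ores, which takes its mesh from a data table row and joins an inventory on Interact.
; ItemDrop stores quantity and item, applies a spawn impulse, then starts a looping slow-down timer.
; The slow-down captures velocity after a delay and lerps it to zero, restarting when a character hits the mesh.
; Overlap pickup is disconnected.
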(event `Drop Slow`
  (bind _item_slow_delay (`self.Item Slow Delay`))
  (bind _item_slow_rate (`self.Item Slow Rate`))
  ; Slow Mesh
  (bind _returnvalue (`KismetSystemLibrary.K2_SetTimerDelegate` (`|CreateDelegate` :!event `Slow Down Drop`) _item_slow_rate true false (`KismetMathLibrary.FClamp` _item_slow_delay (* _item_slow_rate -1.0) _item_slow_delay)))
  (set `self.Item Slow Timer` _returnvalue)
  (`KismetSystemLibrary.Delay` (`self.Item Slow Delay`))
  (set `self.Item Slow Start Velocity` (`SceneComponent.GetComponentVelocity` (`self.Item Mesh`)))
  (set `self.Item Slow Lerp Alpha` 0.0))

(event `ItemDrop`
  (params (Quantity :type Integer) (Item :type "DataTableRowHandle Structure"))
  ; Begin play
  (`self.Set Variables` Quantity Item)
  (`PrimitiveComponent.AddImpulse` (`self.Item Mesh`) (* (`KismetMathLibrary.RandomUnitVector`) (`KismetMathLibrary.RandomFloatInRange` (`self.Min Spawn Impulse`) (`self.Max Spawn Impulse`))) "None" false)
  (`self.Drop Slow`))

(event `self.Sphere.OnComponentBeginOverlap`
  (params (OverlappedComponent :type "PrimitiveComponent Object Reference") (OtherActor :type "Actor Object Reference") (OtherComp :type "PrimitiveComponent Object Reference") (OtherBodyIndex :type Integer) (bFromSweep :type Boolean) (SweepResult :type "HitResult Structure (by ref)"))
  ; Pick Up
  (if (`KismetMathLibrary.ClassIsChildOf` (`GameplayStatics.GetObjectClass` OtherActor) "/Game/Space/Player/BP_TEST_SpaceCharacter.BP_TEST_SpaceCharacter_C")
    _))

(event `/Game/Space/Player/BPI_Interactable.Interact`
  (params (Interactor :type "Pawn Object Reference"))
  ; Pick Up
  (`/Game/Space/ItemSystem/Items/ItemComponent.Add to Inventory` (`self.BP_ItemComponent`) Interactor))

(event `self.Item Mesh.OnComponentHit`
  (params (HitComponent :type "PrimitiveComponent Object Reference") (OtherActor :type "Actor Object Reference") (OtherComp :type "PrimitiveComponent Object Reference") (NormalImpulse :type "Vector Structure") (Hit :type "HitResult Structure (by ref)"))
  (if (`KismetMathLibrary.ClassIsChildOf` (`GameplayStatics.GetObjectClass` OtherActor) "/Game/Space/Player/BP_TEST_SpaceCharacter.BP_TEST_SpaceCharacter_C")
    (`self.Drop Slow`)))

(fn `Get Impulse Values`
  (returns (`Min Impulse` :type "Float (double-precision)") (`Max impulse` :type "Float (double-precision)"))
  (bind _min_spawn_impulse (`self.Min Spawn Impulse`))
  (return (* _min_spawn_impulse -1.0) _min_spawn_impulse))

(fn `Set Variables`
  (params (Quantity :type Integer) (Item :type "DataTableRowHandle Structure"))
  (bind _bp_itemcomponent (`self.BP_ItemComponent`))
  (set `/Game/Space/ItemSystem/Items/ItemComponent.Quantity` Quantity _bp_itemcomponent)
  (bind _output_get (set `/Game/Space/ItemSystem/Items/ItemComponent.Content` Item _bp_itemcomponent))
  (bind _returnvalue (`|GetDataTableRow` (break `DataTableRowHandle` _output_get) (`.RowName` (break `DataTableRowHandle` _output_get)))
    (:`then`
      (`StaticMeshComponent.SetStaticMesh` (`self.Item Mesh`) (`.ItemMesh_19_C1CEC4B44001BCE1DCE588AFED80405C` (break `/Game/Space/ItemSystem/Items/ItemStructure` _returnvalue))))))

(fn `Slow Down Drop`
  (set `self.Item Slow Lerp Alpha` (`KismetMathLibrary.FClamp` (+ (`self.Item Slow Speed`) (`self.Item Slow Lerp Alpha`))))
  (`PrimitiveComponent.SetPhysicsLinearVelocity` (`self.Item Mesh`) (`KismetMathLibrary.VLerp` (`self.Item Slow Start Velocity`) (0.0 0.0 0.0) (`self.Item Slow Lerp Alpha`)) false "None")
  (if (== (`self.Item Slow Lerp Alpha`) 1.0)
    (`KismetSystemLibrary.K2_ClearAndInvalidateTimerHandle` (`self.Item Slow Timer`))))

(fn `UserConstructionScript`)