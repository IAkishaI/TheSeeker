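; Perk manager component that gives its owning actor a random set of perks.
; GeneratePerksSetup picks one class from each of the Heath, Item, Profession and Skill pools, adds it to the owner as a component and records it in ActivePerks.
; The random index uses length minus one as its exclusive maximum, so each pool's last entry is never picked when several exist.
; Progress is printed for debugging.
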(fn `GeneratePerksSetup`
  (bind _heath (`self.Heath`))
  (bind _item (`self.Item`))
  (bind _profession (`self.Profession`))
  (bind _skill (`self.Skill`))
  ; Add perks to owner actor
  (for _array_element (`|MakeArray` (`|GetArrayItem` _heath (`KismetMathLibrary.RandomInteger` (+ (`KismetArrayLibrary.Array_Length` _heath) -1))) (`|GetArrayItem` _item (`KismetMathLibrary.RandomInteger` (+ (`KismetArrayLibrary.Array_Length` _item) -1))) (`|GetArrayItem` _profession (`KismetMathLibrary.RandomInteger` (+ (`KismetArrayLibrary.Array_Length` _profession) -1))) (`|GetArrayItem` _skill (`KismetMathLibrary.RandomInteger` (+ (`KismetArrayLibrary.Array_Length` _skill) -1))))
    (bind _returnvalue (`|AddComponentByClass` (`self.GetOwner`) _array_element))
    (`KismetArrayLibrary.Array_Add` (`self.ActivePerks`) _returnvalue)
    (`KismetSystemLibrary.PrintString` (`KismetSystemLibrary.GetObjectName` _returnvalue)))
  (`KismetSystemLibrary.PrintString` "Complite Generate perk setup"))